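; WallCoverRH is a prototype wall cover actor that detects when an AI arrives at it as its flee destination.
; On overlap, it compares the other actor's FleeToKey blackboard vector with its own location through a tolerance-based Vector Equal macro.
; A match only prints a debug message with that actor's name and location.
; BeginPlay, the construction script and NewFunction_0 are empty.
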(event EventBeginPlay)

(event Collision|EventActorBeginOverlap
  (params (OtherActor :type Actor%20Object%20Reference))
  (Utilities|VectorEqual (AI|Components|Blackboard|GetValueasVector (AI|GetBlackboard OtherActor) (Variables|Default|GetFleeToKey)) (Transformation|GetActorLocation self) 1.0
    (:True
      (Development|PrintString (Utilities|String|ToString(Text) (Utilities|Text|FormatText "{Actor Name} is colliding with me at {Location}" (Utilities|Text|ToText(String) (Utilities|GetDisplayName OtherActor)) (Utilities|Text|ToText(String) (Transformation|GetActorLocation OtherActor))))))))

(fn ConstructionScript)

(fn NewFunction0
  (params (NewParam :type Name) (Inversed :type Boolean)))